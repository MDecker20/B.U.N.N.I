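; BP_Roaming is an AI character that wanders randomly and runs after pawns it sees.
; RandomRoam moves to a random reachable nearby point and calls itself again on success only.
; PawnSensing sightings switch to a run animation and speed and start AIMoveTo on the seen pawn.
; A retriggerable delay, started alongside the chase, restores walking and roaming shortly after sightings stop.
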(event `self.ReceiveBeginPlay`
  (`self.Random Roam`))

(event `Random Roam`
  (`|AIMoveTo` self (`NavigationSystemV1.K2_GetRandomReachablePointInRadius` (`self.K2_GetActorLocation`) 1500.0 null null) null
    (:`OnSuccess`
      (`self.Random Roam`))))

(event `self.PawnSensing.OnSeePawn`
  (params (Pawn :type "Pawn Object Reference"))
  (`|ExecutionSequence`
    (:`then_0`
      (`SkeletalMeshComponent.PlayAnimation` (`self.Mesh`) "/Game/Characters/Mannequins/Animations/Manny/MM_Run_Fwd.MM_Run_Fwd" false)
      (set `CharacterMovementComponent.MaxWalkSpeed` 600.0 (`self.CharacterMovement`)))
    (:`then_1`
      (`|AIMoveTo` self (0.0 0.0 0.0) Pawn
        (:`then`
          (`KismetSystemLibrary.RetriggerableDelay` 2.0)
          (`SkeletalMeshComponent.PlayAnimation` (`self.Mesh`) "/Game/Characters/Mannequins/Animations/Manny/MM_Walk_Fwd.MM_Walk_Fwd" false)
          (set `CharacterMovementComponent.MaxWalkSpeed` 130.0 (`self.CharacterMovement`))
          (`self.Random Roam`))))))

(fn `UserConstructionScript`)