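; Patrol NPC that walks at a reduced speed through a looping route of four PatrolLocation points.
; The GuardPatrol event sets the walk speed and issues AIMoveTo to the point at the Locations index.
; On success it waits a random short delay, calls itself again, and only then increments and wraps the index.
; Move failure is unhandled, and nothing in the graph starts the first patrol.
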(event `Guard Patrol`
  (set `CharacterMovementComponent.MaxWalkSpeed` 150.0 (`self.CharacterMovement`))
  (`|AIMoveTo` self (`|GetArrayItem` (`self.PatrolLocation`) (`self.Locations`)) null
    (:`OnSuccess`
      (`KismetSystemLibrary.Delay` (`KismetMathLibrary.RandomFloatInRange` 1.0 3.0))
      (`self.Guard Patrol`)
      (`/Engine/EditorBlueprintResources/StandardMacros.IncrementInt` (`self.Locations`)
        (:`  `
          (if (== (`self.Locations`) 4)
            (set `self.Locations` 0)))))))

(fn `UserConstructionScript`)